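; Player character Blueprint with Enhanced Input movement, look, jump, hold-to-crouch and hold-to-run, which changes max walk speed.
; On BeginPlay it adds a crosshair widget to the viewport, and F toggles a spotlight flashlight through a FlipFlop.
; Two separate E-key handlers search overlapping BP_Chest actors and send the first interface-implementing one an interaction or open-paper message.
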(event `Key|F`
  (params (Key :type "Key Structure"))
  (bind _spotlight (`self.SpotLight`))
  ; flaslight
  (:`Pressed`
    (`/Engine/EditorBlueprintResources/StandardMacros.FlipFlop`
      (:`A`
        (`LightComponent.SetIntensity` _spotlight 5000.0))
      (:`B`
        (`LightComponent.SetIntensity` _spotlight 0.0)))))

(event `self.ReceiveBeginPlay`
  ; Crosshair
  (bind _returnvalue (`|CreateWidget` "/Game/_Distrora/Widgets/WBP_Crosshair.WBP_Crosshair_C"))
  (`UserWidget.AddToViewport` _returnvalue 0))

(event `EnhancedInput|/Game/_Distrora/input/İnputs/İA_Move`
  (params (ActionValue :type "Vector2D Structure") (ElapsedSeconds :type "Float (double-precision)") (TriggeredSeconds :type "Float (double-precision)") (InputAction :type "InputAction Object Reference" :default "/Game/_Distrora/input/İnputs/İA_Move.İA_Move"))
  (bind (_x _y) (`KismetMathLibrary.BreakVector2D` ActionValue))
  ; Haraket Sistemi
  (:`Triggered`
    (`self.AddMovementInput` (`KismetMathLibrary.GetRightVector` (`self.GetControlRotation`)) _x)
    (`self.AddMovementInput` (`KismetMathLibrary.GetForwardVector` (`self.GetControlRotation`)) _y)))

(event `EnhancedInput|/Game/_Distrora/input/İnputs/İA_Look`
  (params (ActionValue :type "Vector2D Structure") (ElapsedSeconds :type "Float (double-precision)") (TriggeredSeconds :type "Float (double-precision)") (InputAction :type "InputAction Object Reference" :default "/Game/_Distrora/input/İnputs/İA_Look.İA_Look"))
  (bind (_x _y) (`KismetMathLibrary.BreakVector2D` ActionValue))
  ; Bakma Sistemi
  (:`Triggered`
    (`self.AddControllerYawInput` _x)
    (`self.AddControllerPitchInput` _y)))

(event `EnhancedInput|/Game/_Distrora/input/İnputs/İA_JUMP`
  (params (ActionValue :type Boolean) (ElapsedSeconds :type "Float (double-precision)") (TriggeredSeconds :type "Float (double-precision)") (InputAction :type "InputAction Object Reference" :default "/Game/_Distrora/input/İnputs/İA_JUMP.İA_JUMP"))
  ; Zıplama Sistemi
  (:`Started`
    (`self.Jump`))
  (:`Completed`
    (`self.StopJumping`)))

(event `EnhancedInput|/Game/_Distrora/input/İnputs/İA_Crouch`
  (params (ActionValue :type "Vector2D Structure") (ElapsedSeconds :type "Float (double-precision)") (TriggeredSeconds :type "Float (double-precision)") (InputAction :type "InputAction Object Reference" :default "/Game/_Distrora/input/İnputs/İA_Crouch.İA_Crouch"))
  ; Çökme Sistemi
  (:`Started`
    (`self.Crouch`))
  (:`Completed`
    (`self.UnCrouch`)))

(event `EnhancedInput|/Game/_Distrora/input/İnputs/İA_RUN`
  (params (ActionValue :type "Vector2D Structure") (ElapsedSeconds :type "Float (double-precision)") (TriggeredSeconds :type "Float (double-precision)") (InputAction :type "InputAction Object Reference" :default "/Game/_Distrora/input/İnputs/İA_RUN.İA_RUN"))
  ; Koşma Sistemi
  (:`Started`
    (set `CharacterMovementComponent.MaxWalkSpeed` 800.0 (`self.CharacterMovement`)))
  (:`Completed`
    (set `CharacterMovementComponent.MaxWalkSpeed` 450.0 (`self.CharacterMovement`))))

(event `Key|E`
  (params (Key :type "Key Structure"))
  (:`Pressed`
    (for _array_element (`self.GetOverlappingActors` "/Game/_Distrora/Blueprints/etkileşimBluesprint/sandıksal_blu/BP_Chest.BP_Chest_C")
      (if (`KismetSystemLibrary.DoesImplementInterface` _array_element "/Game/_Distrora/Blueprints/etkileşimBluesprint/sandıksal_blu/interactInterFace.interactInterFace_C")
        (message `/Game/_Distrora/Blueprints/etkileşimBluesprint/sandıksal_blu/interactInterFace.InteractWındChesat` _array_element)
        (break)))))

(event `Key|E`
  (params (Key :type "Key Structure"))
  (:`Pressed`
    (for _array_element (`self.GetOverlappingActors` "/Game/_Distrora/Blueprints/etkileşimBluesprint/sandıksal_blu/BP_Chest.BP_Chest_C")
      (if (`KismetSystemLibrary.DoesImplementInterface` _array_element)
        (message `/Game/_Distrora/Player/Bp_Player.openpaper` _array_element)
        (break)))))

(fn `UserConstructionScript`)