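; BP_CashRegister is a cash register prop whose drawer slides open automatically when play begins.
; BeginPlay caches the drawer mesh's relative location as the closed position and derives the open position by offsetting it along local Y.
; The TL_Drawer timeline then plays, lerping the drawer between the two positions through its Alpha track.
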(event `self.ReceiveBeginPlay`
  (set `self.ClosedLoc` (`SceneComponent.RelativeLocation` (`self.CashRegister_011_drawer`)))
  (set `self.OpenLoc` (`KismetMathLibrary.MakeVector` (.x (`self.ClosedLoc`)) (+ (.y (`self.ClosedLoc`)) 27.0) (.z (`self.ClosedLoc`))))
  (bind (_direction _alpha) (`Timeline|TL_Drawer`)
    (:`Update`
      (`SceneComponent.K2_SetRelativeLocation` (`self.CashRegister_011_drawer`) (`KismetMathLibrary.VLerp` (`self.ClosedLoc`) (`self.OpenLoc`) _alpha) false false))))

(fn `UserConstructionScript`)