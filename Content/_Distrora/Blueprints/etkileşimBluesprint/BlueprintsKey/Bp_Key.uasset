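; Key pickup actor that the player collects by pressing E while standing inside its collision volume.
; Overlap by Bp_Player toggles a can-take flag (Anaktarıal) and enables or disables the actor's own input.
; Pressing E with the flag set calls TakeKey, which sets Anahtarvar on the player, prints a Turkish pickup message and destroys the key.
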(event `self.KeyCollision.OnComponentBeginOverlap`
  (params (OverlappedComponent :type "PrimitiveComponent Object Reference") (OtherActor :type "Actor Object Reference") (OtherComp :type "PrimitiveComponent Object Reference") (OtherBodyIndex :type Integer) (bFromSweep :type Boolean) (SweepResult :type "HitResult Structure (by ref)"))
  (cast `/Game/_Distrora/Player/Bp_Player` OtherActor)
  (set `self.anaktarıal` true)
  (`self.EnableInput` (`GameplayStatics.GetPlayerController` 0)))

(event `self.KeyCollision.OnComponentEndOverlap`
  (params (OverlappedComponent :type "PrimitiveComponent Object Reference") (OtherActor :type "Actor Object Reference") (OtherComp :type "PrimitiveComponent Object Reference") (OtherBodyIndex :type Integer))
  (cast `/Game/_Distrora/Player/Bp_Player` OtherActor)
  (set `self.anaktarıal` false)
  (`self.DisableInput` (`GameplayStatics.GetPlayerController` 0)))

(event `TakeKey`
  (bind _asbp_player (cast `/Game/_Distrora/Player/Bp_Player` (`GameplayStatics.GetPlayerCharacter` 0)))
  (set `/Game/_Distrora/Player/Bp_Player.anahtarvar` true _asbp_player)
  (`KismetSystemLibrary.PrintString` "anahtar alındı")
  (`self.K2_DestroyActor`))

(event `Key|E`
  (params (Key :type "Key Structure"))
  (:`Pressed`
    (if (`self.anaktarıal`)
      (`self.TakeKey`))))

(fn `UserConstructionScript`)