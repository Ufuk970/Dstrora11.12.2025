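; BP_RafCekmece is a drawer actor that slides open and closed when the E key is pressed.
; BeginPlay caches the closed location and enables input from player controller 0, with no proximity or aim check on the key.
; Each press toggles IsOpen and plays the TL_Cekmece timeline forward or in reverse, lerping the Çekmece component along relative Y by OpenOffset.
; A Busy flag blocks further presses until the timeline finishes.
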(event `Key|E`
  (params (Key :type "Key Structure"))
  (bind (_closedloc_x _closedloc_y _closedloc_z) (`KismetMathLibrary.BreakVector` (`self.ClosedLoc`)))
  (bind (_openoffset_x _openoffset_y) (`KismetMathLibrary.BreakVector` (`self.OpenOffset`)))
  (:`Pressed`
    (if (not (`self.bBusy`))
      (set `self.bBusy` true)
      (if (`self.bIsOpen`)
        (`|ExecutionSequence`
          (:`then_0`
            (bind (_direction _alpha) (`Timeline|TL_Cekmece` :!via `ReverseFromEnd` :!label _label)
              (:`Update`
                (`SceneComponent.K2_SetRelativeLocation` (`self.çekmece`) (`KismetMathLibrary.VLerp` (`KismetMathLibrary.MakeVector` _closedloc_x _closedloc_y _closedloc_z) (`KismetMathLibrary.MakeVector` _closedloc_x (+ _closedloc_y _openoffset_y) _closedloc_z) _alpha) false false))
              (:`Finished`
                (set `self.bBusy` false))))
          (:`then_1`
            (set `self.bIsOpen` false)))
        (else
          (`|ExecutionSequence`
            (:`then_0`
              (goto _label :!via `PlayFromStart`))
            (:`then_1`
              (set `self.bIsOpen` true))))))))

(event `self.ReceiveBeginPlay`
  (set `self.ClosedLoc` (`SceneComponent.RelativeLocation` (`self.çekmece`)))
  (`self.EnableInput` (`GameplayStatics.GetPlayerController` 0)))

(fn `UserConstructionScript`)